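; Boss enemy that extends a parent AI enemy with a melee weapon and an on-screen health bar.
; The health widget reads the stats component, shows while the boss has a target and hides on death.
; Left and right weapon collision hits apply stat-based point damage to actors that can receive it.
; Combat toggling moves the weapon between hand and attach sockets, and death turns it into a physics object.
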(event `self.ReceiveBeginPlay`
  (`parent.ReceiveBeginPlay`)
  (`/Game/CombatSystem/Blueprints/Components/BP_CollisionComponent.SetCollisionMesh` (`self.RightWeaponCollisionComponent`) (`self.WeaponMesh`))
  (bind _returnvalue (`|CreateWidget` "/Game/CombatSystem/UI/HB_BossHealth.HB_BossHealth_C" (`GameplayStatics.GetPlayerController` 0)))
  (bind _output_get (set `self.BossHealthUI` _returnvalue))
  (`/Game/CombatSystem/UI/HB_BossHealth.Initializate` _output_get (`self.StatsComponent`))
  (`UserWidget.AddToViewport` (`self.BossHealthUI`) 0))

(event `SetBossHealthVisibility`
  (params (`bVisible?` :type Boolean))
  (bind _bosshealthui (`self.BossHealthUI`)
    (:`then`
      (`Widget.SetVisibility` _bosshealthui (select `bool` (and `bVisible?` (not (`/Game/CombatSystem/Blueprints/Components/BP_StateManagerComponent.IsCurrenteStateEqualToAny?` (`self.StateManagerComponent`) (struct :`GameplayTags` (struct :`(TagName` "Character.State.Dead")))))) :`false` "Hidden" :`true` "Visible" :!type "ESlateVisibility Enum")))
    (:`else`)))

(event `self.On Targeted`
  (params (`bIsTargeted?` :type Boolean))
  (`parent.On Targeted` `bIsTargeted?`))

(event `HitEvent`
  (params (`Hit Result` :type "HitResult Structure"))
  (bind (_bblockinghit _binitialoverlap _time _distance _location _impactpoint _normal _impactnormal _physmat _hitactor) (`GameplayStatics.BreakHitResult` `Hit Result`))
  (bind _returnvalue (message `/Game/CombatSystem/Blueprints/Interfaces/Combat_BPI.CanRecieveDamage` _hitactor))
  (if _returnvalue
    (`GameplayStatics.ApplyPointDamage` _hitactor (`/Game/CombatSystem/Blueprints/Components/BP_StatsComponent.GetCurrentStatValue` (`self.StatsComponent`) "NewEnumerator4") (`self.GetActorForwardVector`) `Hit Result` (`self.GetController`) self "/Game/CombatSystem/Blueprints/DamageTypes/BP_AttackDamageType.BP_AttackDamageType_C")))

(event `self.RightWeaponCollisionComponent.OnHit`
  (params (HitResult :type "HitResult Structure"))
  (`self.HitEvent` HitResult))

(event `self.LeftWeaponCollisionComponent.OnHit`
  (params (HitResult :type "HitResult Structure"))
  (`self.HitEvent` HitResult))

(event `SimulateWeaponPhysics`
  (bind _weaponmesh (`self.WeaponMesh`))
  (`PrimitiveComponent.SetCollisionProfileName` _weaponmesh "PhysicsActor" true)
  (`PrimitiveComponent.SetSimulatePhysics` _weaponmesh true))

(event `self.PerformDeath`
  (`parent.PerformDeath`)
  (`self.SimulateWeaponPhysics`)
  (`self.SetBossHealthVisibility` false))

(event `self.CombatComponent.OnCombatToggle`
  (params (`blsCombatEnable?` :type Boolean))
  (`SceneComponent.K2_AttachToComponent` (`self.WeaponMesh`) (`self.Mesh`) (select `bool` `blsCombatEnable?` :`false` (`self.AttachSocketName`) :`true` (`self.WeaponHandSocket`)) "SnapToTarget" "SnapToTarget" "SnapToTarget" true))

(event `self.OnTargetSet`
  (params (NewTarget :type "Actor Object Reference"))
  (`parent.OnTargetSet` NewTarget)
  (`self.SetBossHealthVisibility` (`KismetSystemLibrary.IsValid` NewTarget)))

(fn `UserConstructionScript`
  (`parent.UserConstructionScript`))