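; BP_FrostGiantBoss is the Frost Giant boss character Blueprint in the combat system's AI content.
; On BeginPlay it runs the parent logic, then sets its skeletal mesh as the collision mesh for separate right and left weapon collision components.
; It then plays a character intro montage.
; Tick and overlap events are disabled and the construction script only calls the parent, so this graph adds only startup setup.
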(event `self.ReceiveBeginPlay`
  (bind _mesh (`self.Mesh`))
  (`parent.ReceiveBeginPlay`)
  (`/Game/CombatSystem/Blueprints/Components/BP_CollisionComponent.SetCollisionMesh` (`self.RightWeaponCollisionComponent`) _mesh)
  (`/Game/CombatSystem/Blueprints/Components/BP_CollisionComponent.SetCollisionMesh` (`self.LeftWeaponCollisionComponent`) _mesh)
  (`self.PlayAnimMontage` "/Game/InfinityBladeAdversaries/Enemy/Enemy_Frost_Giant/Enemy_Frost_Giant_All_Animation/FrostGiant_Loop_CharacterIntro_Montage.FrostGiant_Loop_CharacterIntro_Montage"))

(fn `UserConstructionScript`
  (`parent.UserConstructionScript`))