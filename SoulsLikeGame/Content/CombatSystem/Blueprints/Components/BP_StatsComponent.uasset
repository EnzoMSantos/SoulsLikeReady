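; Actor component that stores a combat character's stats in maps keyed by stat, separating base definitions from current values.
; InitializateStats copies each BaseStats entry's base value into CurrentStats.
; ModifyCurrentStatValue adds a non-zero delta and clamps the result between zero and that stat's max, while SetCurrentStatValue writes directly without clamping.
; Getters expose current, base and max values; the event graph is unused.
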(fn `GetBaseStatValue`
  (params (Stat :type "/Game/CombatSystem/Blueprints/Enums/E_Stats Enum" :default "NewEnumerator0"))
  (returns (`Base Value` :type "Float (double-precision)"))
  (return (break `/Game/CombatSystem/Blueprints/Structs/F_BaseTstat` (`BlueprintMapLibrary.Map_Find` (`self.Base Stats`) Stat))))

(fn `GetCurrentStatValue`
  (params (Stat :type "/Game/CombatSystem/Blueprints/Enums/E_Stats Enum" :default "NewEnumerator0"))
  (returns (Value :type "Float (double-precision)"))
  (return (`BlueprintMapLibrary.Map_Find` (`self.Current Stats`) Stat)))

(fn `GetMaxStatValue`
  (params (Stat :type "/Game/CombatSystem/Blueprints/Enums/E_Stats Enum" :default "NewEnumerator0"))
  (returns (Value :type "Float (double-precision)"))
  (return (`.MaxValue_5_2475387F4D528E8B2F80388687036126` (break `/Game/CombatSystem/Blueprints/Structs/F_BaseTstat` (`BlueprintMapLibrary.Map_Find` (`self.Base Stats`) Stat)))))

(fn `InitializateStats`
  (bind _keys (`BlueprintMapLibrary.Map_Keys` (`self.Base Stats`)))
  (for _array_element _keys
    (`self.SetCurrentStatValue` _array_element (break `/Game/CombatSystem/Blueprints/Structs/F_BaseTstat` (`BlueprintMapLibrary.Map_Find` (`self.Base Stats`) _array_element)))))

(fn `ModifyCurrentStatValue`
  (params (Stat :type "/Game/CombatSystem/Blueprints/Enums/E_Stats Enum" :default "NewEnumerator0") (Value :type "Float (double-precision)"))
  (locals (L_Value :type "Float (double-precision)"))
  (if (!= Value 0.0)
    (bind _output_get (set `local.L_Value` (+ (`self.GetCurrentStatValue` (`local.Stat`)) (`local.Value`))))
    (bind _output_get_2 (set `local.L_Value` (`KismetMathLibrary.FClamp` _output_get 0.0 (`self.GetMaxStatValue` (`local.Stat`)))))
    (`self.SetCurrentStatValue` (`local.Stat`) _output_get_2)))

(fn `SetCurrentStatValue`
  (params (Stat :type "/Game/CombatSystem/Blueprints/Enums/E_Stats Enum" :default "NewEnumerator0") (Value :type "Float (double-precision)"))
  (`BlueprintMapLibrary.Map_Add` (`self.Current Stats`) Stat Value))