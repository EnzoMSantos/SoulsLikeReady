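; BP_CollisionComponent is a combat hit-detection component that sweeps for hits along a mesh, between a start and end socket.
; While collision is enabled, Tick runs a multi-sphere object trace between the sockets, skipping ignored actors.
; Each newly hit actor is recorded and broadcast once through OnHit, and enabling collision clears that record for the next activation.
; Setters and getters manage the mesh, ignore list and hit data.
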(event `SetCollisionMesh`
  (params (MeshComponent :type "PrimitiveComponent Object Reference"))
  ;[0.1651 1 0.001518] Set Collision Mesh Component
  (set `self.CollisionMeshComponent` MeshComponent))

(event `EnableCollision`
  ;[0.1651 1 0.001518] Enable/Disable Collision
  (`self.ClearHitActors`)
  (set `self.bIsCollisionEnabled?` true))

(event `DisableCollision`
  ;[0.1651 1 0.001518] Enable/Disable Collision
  (set `self.bIsCollisionEnabled?` false))

(event `ClearHitActors`
  ;[0.1651 1 0.001518] Clear Hit Actors
  (`KismetArrayLibrary.Array_Clear` (`self.AlreadyHitActors`)))

(event `CollisionTrace`
  (bind _collisionmeshcomponent (`self.CollisionMeshComponent`))
  ;[1 0 0] Collision Trace
  (bind _outhits (`KismetSystemLibrary.SphereTraceMultiForObjects` (`SceneComponent.GetSocketLocation` _collisionmeshcomponent (`self.StartSocket Name`)) (`SceneComponent.GetSocketLocation` _collisionmeshcomponent (`self.EndSocket Name`)) (`self.TraceRadius`) (`self.Collision Object Types`) false (`self.Actors to Ignore`) (`self.Draw Debug Type`)))
  (for _array_element _outhits
    (bind _output_get (set `self.LastHit` _array_element))
    (bind (_bblockinghit _binitialoverlap _time _distance _location _impactpoint _normal _impactnormal _physmat _hitactor) (`GameplayStatics.BreakHitResult` _output_get))
    (if (not (`KismetArrayLibrary.Array_Contains` (`self.AlreadyHitActors`) _hitactor))
      (bind _output_get_2 (set `self.Hit Actor` _hitactor))
      (`KismetArrayLibrary.Array_Add` (`self.AlreadyHitActors`) _output_get_2)
      (`self.OnHit` (`self.LastHit`)))))

(event `self.ReceiveTick`
  (params (DeltaSeconds :type "Float (single-precision)"))
  (if (`self.bIsCollisionEnabled?`)
    (`self.CollisionTrace`)))

(fn `AddActorToIgnore`
  (params (InActor :type "Actor Object Reference (by ref)"))
  (`KismetArrayLibrary.Array_AddUnique` (`self.Actors to Ignore`) InActor))

(fn `GetActorsToIgnore`
  (returns (ReturnValue :type "Array of Actor Object Reference"))
  (return (`self.Actors to Ignore`)))

(fn `GetAlreadyHitAcotrs`
  (returns (ReturnValue :type "Array of Actor Object Reference"))
  (return (`self.AlreadyHitActors`)))

(fn `GetCollisionMesh`
  (returns (ReturnValue :type "PrimitiveComponent Object Reference"))
  (return (`self.CollisionMeshComponent`)))

(fn `GetLastHit`
  (returns (ReturnValue :type "HitResult Structure"))
  (return (`self.LastHit`)))

(fn `IsCollisionEnabled?`
  (returns (ReturnValue :type Boolean))
  (return (`self.bIsCollisionEnabled?`)))

(fn `RemoveActorToIgnore`
  (params (InActorToRemove :type "Actor Object Reference (by ref)"))
  (`KismetArrayLibrary.Array_RemoveItem` (`self.Actors to Ignore`) InActorToRemove))