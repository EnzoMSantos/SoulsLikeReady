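; Base weapon Blueprint for the combat system, supplying attack, dodge and combat-toggle montages per gameplay tag, plus action-based stat costs and damage.
; On equip it attaches by combat state, registers as main weapon, updates the owner's anim combat type and feeds its mesh to the collision component.
; Hits on damageable actors apply point damage, with base damage scaled by the current action's multiplier, floored at one.
; An event enables mesh physics for ragdoll.
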(event `self.BP_CollisionComponent.OnHit`
  (params (HitResult :type "HitResult Structure"))
  (bind (_bblockinghit _binitialoverlap _time _distance _location _impactpoint _normal _impactnormal _physmat _hitactor) (`GameplayStatics.BreakHitResult` HitResult))
  ;[0.05127 0.05127 0.05127] Quando hit
  (bind _returnvalue (message `/Game/CombatSystem/Blueprints/Interfaces/Combat_BPI.CanRecieveDamage` _hitactor))
  (if _returnvalue
    (`GameplayStatics.ApplyPointDamage` _hitactor (`self.GetDamage`) (`self.GetActorForwardVector` (`self.GetOwner`)) HitResult (`self.GetInstigatorController`) self)))

(event `SimulateWeaponPhysics`
  (bind _rerutnvalue (`self.GetItemMesh`))
  ;[0.05127 0.05127 0.05127] Fisica da espada quando ativa Ragdoll
  (`PrimitiveComponent.SetCollisionProfileName` _rerutnvalue "PhysicsActor" true)
  (`PrimitiveComponent.SetSimulatePhysics` _rerutnvalue true))

(fn `GetActionMontages`
  (params (`Character Action` :type "GameplayTag Structure"))
  (returns (Montages :type "Array of AnimMontage Object Reference"))
  (`|SwitchGameplayTag` `Character Action`
    (:`Character.Action.Attack.Light Attack`
      (return (`self.LightAttackMontages`)))
    (:`Character.Action.Attack.Heavy Attack`
      (return (`self.HeavyAttackMontages`)))
    (:`Character.Action.Attack.Sprint Attack`
      (return (`self.Sprint Attack`)))
    (:`Character.Action.Attack.Charged Attack`
      (return (`self.Charged Attack`)))
    (:`Character.Action.Attack.Falling Attack`
      (return (`self.Falling Attack`)))
    (:`Character.Action.Dodge`
      (return (`self.DodgeMontages`)))
    (:`Character.Action.Enter Combat`
      (return (`|MakeArray` (`self.EnterCombat`))))
    (:`Character.Action.Exit Combat`
      (return (`|MakeArray` (`self.ExitCombat`))))))

(fn `GetDamage`
  (returns (ReturnValue :type "Float (double-precision)"))
  (bind _ownerstatemanager (`self.OwnerStateManager`)
    (:`then`
      (bind _value (`BlueprintMapLibrary.Map_Find` (`self.ActionDamageMultiplier`) (`/Game/CombatSystem/Blueprints/Components/BP_StateManagerComponent.GetCurrentAction` _ownerstatemanager)))
      (return (* (`self.Damage`) (`KismetMathLibrary.FClamp` _value 1.0 _value))))
    (:`else`
      (return (`self.Damage`)))))

(fn `GetStatCostForAction`
  (returns (Value :type "Float (double-precision)"))
  (bind _ownerstatemanager (`self.OwnerStateManager`)
    (:`then`
      (return (`BlueprintMapLibrary.Map_Find` (`self.ActionStatCost`) (`/Game/CombatSystem/Blueprints/Components/BP_StateManagerComponent.GetCurrentAction` _ownerstatemanager))))
    (:`else`
      (return 0.0))))

(fn `OnEquipped`
  (`parent.OnEquipped`)
  (set `self.CombatCombatComponent` (`self.GetComponentByClass` (`self.GetOwner`) "/Game/CombatSystem/Blueprints/Components/BP_CombatComponent.BP_CombatComponent_C"))
  (set `self.OwnerStateManager` (`self.GetComponentByClass` (`self.GetOwner`) "/Game/CombatSystem/Blueprints/Components/BP_StateManagerComponent.BP_StateManagerComponent_C"))
  (`self.AttachActor` (select `bool` (`/Game/CombatSystem/Blueprints/Components/BP_CombatComponent.IsCombatEnabled?` (`self.CombatCombatComponent`)) :`false` (`self.Attach Socket Name`) :`true` (`self.HandSocketName`)))
  (`/Game/CombatSystem/Blueprints/Components/BP_CombatComponent.SetMainWeapon` (`self.CombatCombatComponent`) self)
  (message `/Game/CombatSystem/Blueprints/Interfaces/AnimInstance_BP.UpdateCombatType` (`SkeletalMeshComponent.GetAnimInstance` (`Character.Mesh` (cast `Character` (`self.GetOwner`) :!pure true))) (`self.CombatType`))
  (`/Game/CombatSystem/Blueprints/Components/BP_CollisionComponent.SetCollisionMesh` (`self.BP_CollisionComponent`) (`self.GetItemMesh`))
  (`/Game/CombatSystem/Blueprints/Components/BP_CollisionComponent.AddActorToIgnore` (`self.BP_CollisionComponent`) (`self.GetOwner`)))

(fn `UserConstructionScript`
  (`parent.UserConstructionScript`))