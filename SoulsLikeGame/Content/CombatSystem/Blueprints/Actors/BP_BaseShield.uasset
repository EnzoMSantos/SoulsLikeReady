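; Base shield equipment actor for the combat system, supplying its own attack, dodge, block and combat-transition montages.
; On equip it attaches to the hand or stowed socket by combat state, binds to combat toggling, and registers as the owner's shield in BP_CombatComponent.
; It also points weapon collision at the item mesh, ignoring the owner; unequipping clears the shield reference.
; GetActionMontages selects montages by character-action gameplay tag.
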(fn `GetActionMontages`
  (params (`Character Action` :type "GameplayTag Structure"))
  (returns (Montages :type "Array of AnimMontage Object Reference"))
  (`|SwitchGameplayTag` `Character Action`
    (:`Character.Action.Attack.Light Attack`
      (return (`self.LightAttackMontages`)))
    (:`Character.Action.Attack.Heavy Attack`
      (return (`self.HeavyAttackMontages`)))
    (:`Character.Action.Attack.Sprint Attack`
      (return (`self.Sprint Attack`)))
    (:`Character.Action.Attack.Charged Attack`
      (return (`self.Charged Attack`)))
    (:`Character.Action.Attack.Falling Attack`
      (return (`self.Falling Attack`)))
    (:`Character.Action.Dodge`
      (return (`self.DodgeMontages`)))
    (:`Character.Action.Enter Combat`
      (return (`|MakeArray` (`self.EnterCombat`))))
    (:`Character.Action.Exit Combat`
      (return (`|MakeArray` (`self.ExitCombat`))))
    (:`Character.Action.Block Attack`
      (return (`self.BlockAnimations`)))))

(fn `OnEquipped`
  (`self.SetIsEquipped` true)
  (`self.AttachActor` (`self.Attach Socket Name`))
  (bind _output_get (set `self.CombatCombatComponent` (`self.GetComponentByClass` (`self.GetOwner`) "/Game/CombatSystem/Blueprints/Components/BP_CombatComponent.BP_CombatComponent_C")))
  (add `/Game/CombatSystem/Blueprints/Components/BP_CombatComponent.OnCombatToggle` _output_get (`|CreateDelegate` :!event `ToggleWeaponCombat`))
  (set `self.OwnerStateManager` (`self.GetComponentByClass` (`self.GetOwner`) "/Game/CombatSystem/Blueprints/Components/BP_StateManagerComponent.BP_StateManagerComponent_C"))
  (`self.AttachActor` (select `bool` (`/Game/CombatSystem/Blueprints/Components/BP_CombatComponent.IsCombatEnabled?` (`self.CombatCombatComponent`)) :`false` (`self.Attach Socket Name`) :`true` (`self.HandSocketName`)))
  (`/Game/CombatSystem/Blueprints/Components/BP_CombatComponent.SetShieldWeapon` (`self.CombatCombatComponent`) self)
  (`/Game/CombatSystem/Blueprints/Components/BP_CollisionComponent.SetCollisionMesh` (`self.MainWeaponCollisionComponent`) (`self.GetItemMesh`))
  (`/Game/CombatSystem/Blueprints/Components/BP_CollisionComponent.AddActorToIgnore` (`self.MainWeaponCollisionComponent`) (`self.GetOwner`)))

(fn `OnUnequipped`
  (`parent.OnUnequipped`)
  (`/Game/CombatSystem/Blueprints/Components/BP_CombatComponent.SetShieldWeapon` (`self.CombatCombatComponent`) null))

(fn `UserConstructionScript`
  (`parent.UserConstructionScript`))