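; Blueprint interface that defines the combat contract for characters in the combat system.
; It declares calls for performing tagged combat actions and attacks, which report success and duration, plus continuing or resetting attacks and combat state.
; Other functions toggle weapon collision by part, i-frames and movement, trigger rotation to a target, and query desired rotation, movement speed mode and whether damage can be received.
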(fn `ActivateCollision`
  (params (CollisionPart :type "/Game/CombatSystem/Blueprints/Enums/E_CollisionPart Enum" :default "NewEnumerator0")))

(fn `CanRecieveDamage`
  (returns (ReturnValue :type Boolean))
  (return false))

(fn `ContinueAttack`
  (return))

(fn `DeactivateCollision`
  (params (CollisionPart :type "/Game/CombatSystem/Blueprints/Enums/E_CollisionPart Enum" :default "NewEnumerator0")))

(fn `GetDesiredRotation`
  (returns (ReturnValue :type "Rotator Structure"))
  (return))

(fn `GetMovementSpeedMode`
  (returns (ReturnValue :type "/Game/CombatSystem/Blueprints/Enums/E_MovementSpeedMode Enum"))
  (return "NewEnumerator0"))

(fn `Perform Combat Action`
  (params (ActionTag :type "GameplayTag Structure") (StateTag :type "GameplayTag Structure" :default (struct :`TagName` "Character.State.General Action State")) (MontageIndex :type Integer) (RandomIndex :type Boolean))
  (returns (`Sucess?` :type Boolean) (ActionDuration :type "Float (double-precision)"))
  (return false 0.0))

(fn `PerformCombatAttack`
  (params (AttackType :type "GameplayTag Structure") (AttackIndex :type Integer) (RandomIndex :type Boolean))
  (returns (`Sucess?` :type Boolean) (AttackDuration :type "Float (double-precision)"))
  (return false 0.0))

(fn `ResetAttack`)

(fn `ResetCombat`)

(fn `RotateToTarget`)

(fn `SetCanMove`
  (params (`bCanMove?` :type Boolean)))

(fn `SetIframes`
  (params (bEnabledIFrames :type Boolean)))